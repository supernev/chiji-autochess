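; BP_Fighter is the fighter actor Blueprint for the ChijiAutoChess auto-chess game.
; On BeginPlay it casts the Bar widget component's user widget to WGP_Fighter_Bar and sets itself as that bar's OwnerFighter.
; StandInLocation places the fighter at a given point, raised by the capsule half-height so the capsule rests on that spot.
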(event `self.ReceiveBeginPlay`
  (bind _aswgp_fighter_bar (cast `/Game/ChijiAutoChess/Fighters/WGP_Fighter_Bar` (`WidgetComponent.GetUserWidgetObject` (`self.Bar`))))
  (set `/Game/ChijiAutoChess/Fighters/WGP_Fighter_Bar.OwnerFighter` self _aswgp_fighter_bar))

(fn `StandInLocation`
  (params (Location :type "Vector Structure"))
  (`self.K2_SetActorLocation` self (`KismetMathLibrary.MakeVector` Location_X Location_Y (+ Location_Z (`CapsuleComponent.CapsuleHalfHeight` (`self.CapsuleComponent`)))) false false))

(fn `UserConstructionScript`)