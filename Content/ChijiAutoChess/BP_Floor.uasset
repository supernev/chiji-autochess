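; BP_Floor is the board actor for the ChijiAutoChess game, holding fighters in a Grids array of slots.
; On BeginPlay it resizes Grids to 100 entries.
; PlaceFighter stores a fighter at a slot index and teleports it to a world location from CalcLocation, which lays slots in a single line along Y at fixed spacing, independent of the floor's own transform.
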(event `self.ReceiveBeginPlay`
  (`KismetArrayLibrary.Array_Resize` (`self.Grids`) 100))

(fn `CalcLocation`
  (params (Position :type Integer))
  (returns (Location :type "Vector Structure"))
  (return (`KismetMathLibrary.MakeVector` 0.0 (* Position 10.0))))

(fn `PlaceFighter`
  (params (Fighter :type "/Game/ChijiAutoChess/Fighters/BP_Fighter Object Reference") (Position :type Integer))
  (`KismetArrayLibrary.Array_Set` (`self.Grids`) Position Fighter)
  (bind _location (`self.CalcLocation` Position))
  (`self.K2_SetActorLocation` Fighter _location false true)
  (return))

(fn `UserConstructionScript`)